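; Portal component that shows visual clones of its owner at the linked portal while the owner overlaps one.
; On BeginPlay it spawns collisionless clones of visible static and skeletal meshes, using master pose for skeletal ones.
; Post-update tick moves them through the portal's transform and toggles visibility.
; While touching, it disables collision with both portals' blocking walls, using spawned physics constraints for rigid bodies and move-ignore for capsules.
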(event `self.ReceiveBeginPlay`
  (bind _returnvalue (== (`self.Owner Actor`) (`GameplayStatics.GetPlayerPawn` 0)))
  (`|ExecutionSequence`
    (:`then_0`
      ;[0 0.6377 0.1836] tick after physics
      (`self.SetTickGroup` "TG_PostUpdateWork"))
    (:`then_1`
      ;;[0 0.2126 0.6087] set owner
      (bind _output_get (set `self.Owner Actor` (`self.GetOwner`)))
      ;;;[0 0.4445 0.3768] Handle Destroying actor
      (add `Actor.OnDestroyed` _output_get (delegate `Event Destroy Clone Actors`))
      ;;;;[0.1932 0 0.6355] clone actor
      (`self.GenerateClones`))
    (:`then_2`
      (if _returnvalue
        (set `self.OwnerActorIsPlayerPawn` _returnvalue)))))

(event `Event Destroy Clone Actors`
  (params (DestroyedActor :type "Actor Object Reference"))
  ;[0 0.6377 0.1836] tick after physics
  ;;[0 0.2126 0.6087] set owner
  ;;;[0 0.4445 0.3768] Handle Destroying actor
  (`self.DestroyCloneActors`))

(event `self.ReceiveTick`
  (params (DeltaSeconds :type "Float (single-precision)"))
  (bind _attached_clone_actors_dict (`self.attached_clone_actors_dict`))
  (set `self.WasTouchingPortal` (`self.TouchingPortal`))
  ;[0 0.1643 0.657] overlapping a portal? (could do loop insted of check elem 0)
  (bind _output_get (set `self.overlapping` (`Actor.GetOverlappingActors` (`self.Owner Actor`) "/Game/PortalsBP/Blueprints/PortalBP.PortalBP_C")))
  (if (> (`KismetArrayLibrary.Array_Length` _output_get) 0)
    (bind _asportal_bp (cast `/Game/PortalsBP/Blueprints/PortalBP` (`|GetArrayItem` _output_get))
      (:`then`
        (set `self.overlapped_portal` _asportal_bp)
        (set `self.TouchingPortal` true)
        (`|ExecutionSequence`
          (:`then_0`
            ;[0 0.8116 0.009662] Set position of visual portal clone
            (bind _keys (`BlueprintMapLibrary.Map_Keys` _attached_clone_actors_dict))
            (for _array_element _keys
              (bind _transform_out (`/Game/PortalsBP/Blueprints/PortalTickComponent.ChangeTransform` (`/Game/PortalsBP/Blueprints/PortalBP.PortalTickComponent` (`self.overlapped_portal`)) (`SceneComponent.K2_GetComponentToWorld` _array_element)))
              (`Actor.K2_SetActorTransform` (`BlueprintMapLibrary.Map_Find` _attached_clone_actors_dict _array_element) _transform_out false false)))
          (:`then_1`
            ;;[0 0.3382 0.4831] show if touching a portal
            (`self.set_actors_hidden` false))
          (:`then_2`
            ;[0.4445 0 0.3813] Disable collision
            (if (not (`self.WasTouchingPortal`))
              (`self.DisableCollision`)))))
      (:`CastFailed`
        ;[0.6764 0 0.1467] hide if not touching portals
        (`self.set_actors_hidden` true :!label _label)
        (set `self.TouchingPortal` false)
        ;[0 0.3865 0.4348] enable collision
        (if (`self.WasTouchingPortal`)
          (`self.EnableCollision`))))
    (else
      (goto _label))))

(event `DisableCollision`
  (bind _overlapped_portal (`self.overlapped_portal`))
  (bind _overlapped_portal_2 (`self.overlapped_portal`))
  (bind _rootcomponent (`Actor.RootComponent` (`self.Owner Actor`)))
  (bind _blockingwall (`/Game/PortalsBP/Blueprints/PortalBP.BlockingWall` _overlapped_portal))
  (bind _blockingwall_2 (`/Game/PortalsBP/Blueprints/PortalBP.BlockingWall` _overlapped_portal_2))
  (bind _blockingwall_3 (`/Game/PortalsBP/Blueprints/PortalBP.BlockingWall` (`/Game/PortalsBP/Blueprints/PortalBP.TargetPortal` _overlapped_portal)))
  (bind _blockingwall_4 (`/Game/PortalsBP/Blueprints/PortalBP.BlockingWall` (`/Game/PortalsBP/Blueprints/PortalBP.TargetPortal` _overlapped_portal_2)))
  ;[0 0.4831 0.3382] disable collision with object behind portal
  (bind _returnvalue (`|SpawnActorFromClass` "/Game/PortalsBP/Blueprints/portal_CollisionDisabler.portal_CollisionDisabler_C" (`KismetMathLibrary.MakeTransform` (0.0 0.0 0.0)) "Undefined" "OverrideRootScale" null null))
  (set `self.collision_disabler` _returnvalue)
  (`|ExecutionSequence`
    (:`then_0`
      (bind _asprimitive_component (cast `PrimitiveComponent` _rootcomponent))
      ;;[0 0.3382 0.4831] constraints disable collision for rigidbodys
      (`|ExecutionSequence`
        (:`then_0`
          (`/Engine/EditorBlueprintResources/StandardMacros.IsValid` _blockingwall_3
            (:`Is Valid`
              (`PhysicsConstraintComponent.SetConstrainedComponents` (`/Game/PortalsBP/Blueprints/portal_CollisionDisabler.PhysicsConstraint` (`self.collision_disabler`)) _asprimitive_component "None" _blockingwall_3 "None"))))
        (:`then_1`
          (`/Engine/EditorBlueprintResources/StandardMacros.IsValid` _blockingwall
            (:`Is Valid`
              (`PhysicsConstraintComponent.SetConstrainedComponents` (`/Game/PortalsBP/Blueprints/portal_CollisionDisabler.PhysicsConstraint1` (`self.collision_disabler`)) _asprimitive_component "None" _blockingwall "None"))))))
    (:`then_1`
      (bind _ascapsule_collision (cast `CapsuleComponent` _rootcomponent))
      (`|ExecutionSequence`
        (:`then_0`
          (`/Engine/EditorBlueprintResources/StandardMacros.IsValid` _blockingwall_4
            (:`Is Valid`
              (`PrimitiveComponent.IgnoreActorWhenMoving` _ascapsule_collision (`self.GetOwner` _blockingwall_4) true))))
        (:`then_1`
          (`/Engine/EditorBlueprintResources/StandardMacros.IsValid` _blockingwall_2
            (:`Is Valid`
              (`PrimitiveComponent.IgnoreActorWhenMoving` _ascapsule_collision (`self.GetOwner` _blockingwall_2) true))))))))

(event `EnableCollision`
  (bind _overlapped_portal (`self.overlapped_portal`))
  (bind _blockingwall (`/Game/PortalsBP/Blueprints/PortalBP.BlockingWall` _overlapped_portal))
  (bind _blockingwall_2 (`/Game/PortalsBP/Blueprints/PortalBP.BlockingWall` (`/Game/PortalsBP/Blueprints/PortalBP.TargetPortal` _overlapped_portal)))
  ;[0.3672 0.4541 0] re-enable collision
  (`|ExecutionSequence`
    (:`then_0`
      (bind _ascapsule_collision (cast `CapsuleComponent` (`Actor.RootComponent` (`self.Owner Actor`))))
      (`PrimitiveComponent.ClearMoveIgnoreComponents` _ascapsule_collision)
      (`|ExecutionSequence`
        (:`then_0`
          (`/Engine/EditorBlueprintResources/StandardMacros.IsValid` _blockingwall_2
            (:`Is Valid`
              (`PrimitiveComponent.IgnoreActorWhenMoving` _ascapsule_collision (`self.GetOwner` _blockingwall_2) false))))
        (:`then_1`
          (`/Engine/EditorBlueprintResources/StandardMacros.IsValid` _blockingwall
            (:`Is Valid`
              (`PrimitiveComponent.IgnoreActorWhenMoving` _ascapsule_collision (`self.GetOwner` _blockingwall) false))))))
    (:`then_1`
      (`Actor.K2_DestroyActor` (`self.collision_disabler`)))))

(fn `DestroyCloneActors`
  (`|ExecutionSequence`
    (:`then_0`
      ;[0 0.6764 0.1449] destroy actors
      (for _array_element (`self.attached_clone_actors`)
        (`Actor.K2_DestroyActor` _array_element)))
    (:`then_1`
      ;;[0.1739 0 0.6551] clear clone actors dict and list
      (`KismetArrayLibrary.Array_Clear` (`self.attached_clone_actors`))
      (`BlueprintMapLibrary.Map_Clear` (`self.attached_clone_actors_dict`)))))

(fn `GenerateClones`
  ;[0.1063 0 0.7235] skel
  ;;[0.7054 0 0.1173] static
  (`|ExecutionSequence`
    (:`then_0`
      (for _array_element (`Actor.K2_GetComponentsByClass` (`self.Owner Actor`) "/Script/Engine.SkeletalMeshComponent")
        (`self.GenerateSkeletalClones` _array_element)))
    (:`then_1`
      (for _array_element_2 (`Actor.K2_GetComponentsByClass` (`self.Owner Actor`) "/Script/Engine.StaticMeshComponent")
        (`self.GenerateStaticMeshClones` _array_element_2)))))

(fn `GenerateSkeletalClones`
  (params (SkeletalMeshComponent :type "SkeletalMeshComponent Object Reference"))
  (locals (target_skel_mesh_component :type "SkeletalMeshComponent Object Reference") (target_skel_mesh :type "SkeletalMesh Object Reference") (cloned_skel_component :type "SkeletalMeshComponent Object Reference") (cloned_skel :type "/Game/PortalsBP/Blueprints/portal_clone_skeletal Object Reference"))
  (bind _cloned_skel_component (`local.cloned_skel_component`))
  (`|ExecutionSequence`
    (:`then_0`
      ;[0 0.4541 0.3672] setup vars
      (bind _output_get (set `local.target_skel_mesh_component` SkeletalMeshComponent))
      (set `local.target_skel_mesh` (`SkinnedMeshComponent.SkeletalMesh` _output_get)))
    (:`then_1`
      ;[0 0.5701 0.2512] filter visible
      (if (`SceneComponent.IsVisible` (`local.target_skel_mesh_component`))
        (`|ExecutionSequence`
          (:`then_0`
            ;[0 0.5508 0.2705] create skel actor, add to list and dict
            (bind _returnvalue (`|SpawnActorFromClass` "/Game/PortalsBP/Blueprints/portal_clone_skeletal.portal_clone_skeletal_C" (`SceneComponent.K2_GetComponentToWorld` (`local.target_skel_mesh_component`)) "AlwaysSpawn" "OverrideRootScale" null null))
            (bind _output_get_2 (set `local.cloned_skel` _returnvalue))
            (set `local.cloned_skel_component` (`/Game/PortalsBP/Blueprints/portal_clone_skeletal.SkeletalMesh` _output_get_2))
            (`KismetArrayLibrary.Array_Add` (`self.attached_clone_actors`) (`local.cloned_skel`))
            (`BlueprintMapLibrary.Map_Add` (`self.attached_clone_actors_dict`) (`local.target_skel_mesh_component`) (`local.cloned_skel`)))
          (:`then_1`
            ;[0.1159 0 0.7138] attach skel mesh, disable collision
            (`SceneComponent.K2_AttachTo` (`local.cloned_skel_component`) (`local.target_skel_mesh_component`) "None" "SnapToTargetIncludingScale" false)
            (`SkinnedMeshComponent.SetSkinnedAssetAndUpdate` (`local.cloned_skel_component`) (`local.target_skel_mesh`) true)
            (`PrimitiveComponent.SetCollisionEnabled` (`local.cloned_skel_component`) "NoCollision"))
          (:`then_3`
            ;[0.5218 0 0.3031] match parents pose
            (`SkinnedMeshComponent.SetLeaderPoseComponent` (`local.cloned_skel_component`) (`local.target_skel_mesh_component`) false))
          (:`then_4`
            ;[0.773 0 0.04889] use abs location
            (set `SceneComponent.bAbsoluteLocation` true _cloned_skel_component)
            (set `SceneComponent.bAbsoluteRotation` true _cloned_skel_component)
            ;[0 0.715 0.1063] set better world location+rot
            (`SceneComponent.K2_SetWorldLocationAndRotation` (`local.cloned_skel_component`) (.location (`SceneComponent.K2_GetComponentToWorld` (`local.target_skel_mesh_component`))) (.rotation (`SceneComponent.K2_GetComponentToWorld` (`local.target_skel_mesh_component`))) false false)))
        (else
          (return))))))

(fn `GenerateStaticMeshClones`
  (params (StaticMeshComponent :type "StaticMeshComponent Object Reference"))
  (locals (target_mesh_component :type "StaticMeshComponent Object Reference") (cloned_mesh_component :type "StaticMeshComponent Object Reference") (target_mesh :type "StaticMesh Object Reference") (cloned_mesh :type "/Game/PortalsBP/Blueprints/portal_clone_static_mesh Object Reference"))
  (bind _owner_actor (`self.Owner Actor`))
  (bind _cloned_mesh (`local.cloned_mesh`))
  (bind _cloned_mesh_component (`local.cloned_mesh_component`))
  (`|ExecutionSequence`
    (:`then_0`
      ;[0.773 0.04831 0] setup vars
      (bind _output_get (set `local.target_mesh_component` StaticMeshComponent))
      (set `local.target_mesh` (`StaticMeshComponent.StaticMesh` _output_get)))
    (:`then_1`
      ;[0 0.7054 0.1159] filter visible
      (if (`SceneComponent.IsVisible` (`local.target_mesh_component`))
        (`|ExecutionSequence`
          (:`then_0`
            ;[0 0.4735 0.3478] create actor, add to list and dict
            (bind _returnvalue (`|SpawnActorFromClass` "/Game/PortalsBP/Blueprints/portal_clone_static_mesh.portal_clone_static_mesh_C" (`Actor.GetTransform` _owner_actor) "AlwaysSpawn" "OverrideRootScale" _owner_actor null))
            (bind _output_get_2 (set `local.cloned_mesh` _returnvalue))
            (set `local.cloned_mesh_component` (`/Game/PortalsBP/Blueprints/portal_clone_static_mesh.StaticMesh` _output_get_2))
            (`KismetArrayLibrary.Array_Add` (`self.attached_clone_actors`) _cloned_mesh)
            (`BlueprintMapLibrary.Map_Add` (`self.attached_clone_actors_dict`) (`local.target_mesh_component`) _cloned_mesh))
          (:`then_1`
            ;[0.6184 0 0.2053] attach mesh, disable collision
            (`SceneComponent.K2_AttachTo` (`local.cloned_mesh_component`) (`local.target_mesh_component`) "None" "SnapToTargetIncludingScale" false)
            (`StaticMeshComponent.SetStaticMesh` (`local.cloned_mesh_component`) (`local.target_mesh`))
            (`PrimitiveComponent.SetCollisionEnabled` (`local.cloned_mesh_component`) "NoCollision"))
          (:`then_2`
            ;[0.4541 0 0.3715] use abs location
            (set `SceneComponent.bAbsoluteLocation` true _cloned_mesh_component)
            (set `SceneComponent.bAbsoluteRotation` true _cloned_mesh_component)
            ;[0.4928 0.3285 0] set better world location+rot
            (`SceneComponent.K2_SetWorldLocationAndRotation` (`local.cloned_mesh_component`) (.location (`SceneComponent.K2_GetComponentToWorld` (`local.target_mesh_component`))) (.rotation (`SceneComponent.K2_GetComponentToWorld` (`local.target_mesh_component`))) false false))
          (:`then_3`
            ;[0 0.715 0.1063] set material
            (for (_ _array_index) (`MeshComponent.GetMaterials` (`local.cloned_mesh_component`))
              (`PrimitiveComponent.SetMaterial` (`local.cloned_mesh_component`) _array_index (`PrimitiveComponent.GetMaterial` (`local.target_mesh_component`) _array_index)))))))))

(fn `set_actors_hidden`
  (params (bNewHidden :type Boolean))
  (for _array_element (`self.attached_clone_actors`)
    (`Actor.SetActorHiddenInGame` _array_element bNewHidden)))